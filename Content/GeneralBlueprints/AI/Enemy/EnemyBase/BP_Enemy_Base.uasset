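; Base enemy Character Blueprint that supplies shared movement and query functions for AI enemies.
; JumptoDestination launches the character with a suggested custom-arc velocity toward a point slightly above the target.
; SetMovementSpeed maps a speed state to max walk speed, and GetPatrolRoute returns the assigned route.
; Health, heal and death functions are stubs returning defaults, and the damage system component is unused here.
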(event `/Game/GeneralBlueprints/AI/Enemy/EnemyBase/BPI_EnemyAI.JumpToDestination`
  (params (Destination :type "Vector Structure"))
  (bind _outlaunchvelocity (`GameplayStatics.SuggestProjectileVelocity_CustomArc` (`self.K2_GetActorLocation`) (`KismetMathLibrary.MakeVector` (.x Destination) (.y Destination) (+ (.z Destination) 75.0))))
  (`self.LaunchCharacter` _outlaunchvelocity true true))

(fn `GetCurrentHealth`
  (returns (Health :type "Float (double-precision)"))
  (return 0.0))

(fn `GetMaxHealth`
  (returns (Health :type "Float (double-precision)"))
  (return 0.0))

(fn `GetPatrolRoute`
  (returns (PatrolRoute :type "/Game/GeneralBlueprints/AI/BP_PatrolRoute Object Reference"))
  (return (`self.PatrolRoute`)))

(fn `Heal`
  (params (HealAmount :type "Float (double-precision)"))
  (returns (NewHealth :type "Float (double-precision)"))
  (return 0.0))

(fn `IsDead`
  (returns (IsDead :type Boolean))
  (return false))

(fn `SetMovementSpeed`
  (params (Speed :type "/Game/GeneralBlueprints/AI/Enums/E_AISpeed Enum" :default "NewEnumerator0"))
  (returns (SpeedValue :type "Float (double-precision)"))
  (bind _output_get (set `CharacterMovementComponent.MaxWalkSpeed` (select `/Game/GeneralBlueprints/AI/Enums/E_AISpeed` Speed :`NewEnumerator1` 300.0 :`NewEnumerator2` 360.0 :`NewEnumerator3` 550.0 :!type "Float (single-precision)") (`self.CharacterMovement`)))
  (return _output_get))

(fn `UserConstructionScript`)