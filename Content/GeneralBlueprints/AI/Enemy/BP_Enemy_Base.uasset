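; Base enemy character Blueprint providing attack, jump, patrol route and movement speed functionality for enemy AI.
; Attack plays a montage, kills the first-person player on completion without a range check, and fires OnAttackEnd afterwards or on interruption.
; JumptoDestination launches the character on a computed projectile arc to just above the target.
; SetMovementSpeed maps an Idle-to-Sprinting enum to walk speed, and GetPatrolRoute exposes the assigned route.
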(event `self.ReceiveBeginPlay`)

(event `Attack`
  (`|PlayMontage` (`self.Mesh`) "/Game/Assets/Characters/Mannequins/Animations/Manny/AM_TestAnim.AM_TestAnim"
    (:`OnCompleted`
      (bind _asbp_first_person_character (cast `/Game/FirstPerson/Blueprints/BP_FirstPersonCharacter` (`GameplayStatics.GetPlayerCharacter` 0)))
      (`/Game/FirstPerson/Blueprints/BP_FirstPersonCharacter.DIE` _asbp_first_person_character))
    (:`OnInterrupted`
      _))
  (`self.OnAttackEnd`))

(event `/Game/GeneralBlueprints/AI/BPI_EnemyAI.JumpToDestination`
  (params (Destination :type "Vector Structure"))
  (bind _outlaunchvelocity (`GameplayStatics.SuggestProjectileVelocity_CustomArc` (`self.K2_GetActorLocation`) (`KismetMathLibrary.MakeVector` (.x Destination) (.y Destination) (+ (.z Destination) 75.0))))
  (`self.LaunchCharacter` _outlaunchvelocity true true))

(fn `GetPatrolRoute`
  (returns (PatrolRoute :type "/Game/GeneralBlueprints/AI/BP_PatrolRoute Object Reference"))
  (return (`self.PatrolRoute`)))

(fn `SetMovementSpeed`
  (params (Speed :type "/Game/GeneralBlueprints/AI/Enums/E_AISpeed Enum" :default "NewEnumerator0"))
  (returns (SpeedValue :type "Float (double-precision)"))
  (bind _output_get (set `CharacterMovementComponent.MaxWalkSpeed` (select `/Game/GeneralBlueprints/AI/Enums/E_AISpeed` Speed :`NewEnumerator1` 200.0 :`NewEnumerator2` 300.0 :`NewEnumerator3` 450.0 :!type "Float (single-precision)") (`self.CharacterMovement`)))
  (return _output_get))

(fn `UserConstructionScript`)