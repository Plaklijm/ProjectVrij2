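; BP_PatrolEnemy is an enemy character whose attack lunges through the player, phasing past pawn collision.
; Attack sets pawn collision to overlap, launches along velocity with a hop and then along its facing, and calls JuiceChunk on the player.
; After a short delay it restores blocking and signals the attack's end.
; Any overlap with the first-person character calls HitByPhaseEnemy on it.
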(event `/Game/GeneralBlueprints/AI/Enemy/EnemyBase/BPI_EnemyAI.Attack`
  (params (Player :type "/Game/FirstPerson/Blueprints/BP_FirstPersonCharacter Object Reference"))
  (bind (_returnvalue_x _returnvalue_y) (`KismetMathLibrary.BreakVector` (* (`self.GetVelocity`) 200.0)))
  (set `self.IsAttacking` true)
  (`KismetSystemLibrary.Delay` 0.075)
  (`PrimitiveComponent.SetCollisionResponseToChannel` (`self.CapsuleComponent`) "ECC_Pawn" "ECR_Overlap")
  (`KismetSystemLibrary.Delay` 0.05)
  (`self.LaunchCharacter` (`KismetMathLibrary.MakeVector` _returnvalue_x _returnvalue_y 150.0))
  (`KismetSystemLibrary.Delay` 0.05)
  (`self.LaunchCharacter` (* (`KismetMathLibrary.GetForwardVector` (`self.K2_GetActorRotation`)) 1000.0))
  (`HorrorTemplateCharacter.JuiceChunk` Player (`self.JuiceChunkAmount`))
  (set `self.IsAttacking` false)
  (`KismetSystemLibrary.Delay` 0.7)
  (`PrimitiveComponent.SetCollisionResponseToChannel` (`self.CapsuleComponent`) "ECC_Pawn" "ECR_Block")
  (`self.OnAttackEnd`))

(event `self.ReceiveActorBeginOverlap`
  (params (OtherActor :type "Actor Object Reference"))
  (bind _asbp_first_person_character (cast `/Game/FirstPerson/Blueprints/BP_FirstPersonCharacter` OtherActor))
  (`/Game/FirstPerson/Blueprints/BP_FirstPersonCharacter.HitByPhaseEnemy` _asbp_first_person_character))

(fn `UserConstructionScript`
  (`parent.UserConstructionScript`))