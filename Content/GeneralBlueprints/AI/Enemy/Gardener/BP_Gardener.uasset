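; BP_Gardener is an enemy that starts frozen in a slump, then stands and seeks the player.
; A timeline polls controller line of sight; the first sighting triggers stand-up, then AIC_Gardener seeks the player's location.
; A gate closed by sighting lets an unseen Gardener request a respawn through the player and destroy itself when the timeline ends.
; Attack notifies the caught player, plays a grab montage, then kills them and signals attack end.
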(event `self.ReceiveBeginPlay`
  (bind _returnvalue (`GameplayStatics.GetPlayerCharacter` 0))
  (`parent.ReceiveBeginPlay`)
  (bind _asaic_gardener (cast `/Game/GeneralBlueprints/AI/Enemy/Gardener/AIC_Gardener` (`self.GetController`)))
  (`/Game/GeneralBlueprints/AI/Enemy/EnemyBase/AIC_Enemy_Base.SetStateAsFrozen` _asaic_gardener)
  (`|PlayMontage` (`self.Mesh`) "/Game/Assets/Characters/Mannequins/Animations/Manny/AS_NAAT_Zombie_SlumpToStandCONVERTED_Montage.AS_NAAT_Zombie_SlumpToStandCONVERTED_Montage" 1.0 0.0 "Default"
    (:`then`
      (`Timeline|Timeline` :!via `PlayFromStart`
        (:`Update`
          (if (`Controller.LineOfSightTo` (`self.GetController`) _returnvalue (0.0 0.0 0.0) false)
            (`/Engine/EditorBlueprintResources/StandardMacros.DoOnce` false
              (:`Completed`
                (`|PlayMontage` (`self.Mesh`) "/Game/Assets/Characters/Mannequins/Animations/Manny/AS_NAAT_Zombie_SlumpToStandCONVERTED_Montage.AS_NAAT_Zombie_SlumpToStandCONVERTED_Montage" 1.0 0.0 "StandUp"
                  (:`then`
                    (goto _label :!via `Close`))
                  (:`OnCompleted`
                    _)
                  (:`OnInterrupted`
                    _))
                (bind _asaic_gardener_2 (cast `/Game/GeneralBlueprints/AI/Enemy/Gardener/AIC_Gardener` (`self.GetController`)))
                (`/Game/GeneralBlueprints/AI/Enemy/EnemyBase/AIC_Enemy_Base.SetStateAsSeeking` _asaic_gardener_2 (`self.K2_GetActorLocation` (`GameplayStatics.GetPlayerCharacter` 0)))))))
        (:`Finished`
          (`/Engine/EditorBlueprintResources/StandardMacros.Gate` false :!label _label
            (:`Exit`
              (bind _asbp_first_person_character (cast `/Game/FirstPerson/Blueprints/BP_FirstPersonCharacter` _returnvalue))
              (`/Game/FirstPerson/Blueprints/BP_FirstPersonCharacter.TrySpawnGardener` _asbp_first_person_character)
              (`self.K2_DestroyActor`))))))))

(event `/Game/GeneralBlueprints/AI/Enemy/EnemyBase/BPI_EnemyAI.Attack`
  (params (Player :type "/Game/FirstPerson/Blueprints/BP_FirstPersonCharacter Object Reference"))
  (`/Game/FirstPerson/Blueprints/BP_FirstPersonCharacter.GardenerCatch` Player self)
  (`KismetSystemLibrary.Delay` 0.2)
  (`|PlayMontage` (`self.Mesh`) "/Game/Assets/Characters/Mannequins/Animations/Manny/AS_NAAT_Zombie_Idle_To_Grab1_Montage.AS_NAAT_Zombie_Idle_To_Grab1_Montage"
    (:`OnCompleted`
      _)
    (:`OnInterrupted`
      _))
  (`/Game/FirstPerson/Blueprints/BP_FirstPersonCharacter.DIE` Player)
  (`self.OnAttackEnd`))

(fn `UserConstructionScript`
  (`parent.UserConstructionScript`))