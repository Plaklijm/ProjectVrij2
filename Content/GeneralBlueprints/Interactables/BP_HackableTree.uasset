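; Interactable tree that the first-person player can push over once, despite the "Hackable" name.
; On Interact, a timeline glides the player to a preset position and facing, then calls PushTreeDown on the character.
; After a delay timed to the push, it plays the fall sound and a second timeline rotates the root pivot.
; Landing sets TreeDown and triggers camera shake and force feedback at the player.
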(event `self.ReceiveTick`
  (params (DeltaSeconds :type "Float (single-precision)"))
  (if (`self.TreeDown`)
    _))

(event `InteractInterface.Interact`
  (params (player :type "HorrorTemplateCharacter Object Reference") (ElapsedSeconds :type "Float (single-precision)"))
  (bind _returnvalue (`self.GetTransform` player))
  (bind _returnvalue_2 (`self.K2_GetActorLocation` (`GameplayStatics.GetPlayerCharacter` 0)))
  (bind _returnvalue_3 (`SceneComponent.K2_GetComponentToWorld` (`self.PlayerPosition_0`)))
  (`/Engine/EditorBlueprintResources/StandardMacros.DoOnce` false
    (:`Completed`
      (if (not (`self.TreeDown`))
        (bind (_direction _time) (`Timeline|MovePLayer` :!via `PlayFromStart`)
          (:`Update`
            (bind (_returnvalue_x _returnvalue_y) (`KismetMathLibrary.BreakVector` (`KismetMathLibrary.VInterpTo_Constant` (`KismetMathLibrary.MakeVector` (.x (.location _returnvalue)) (.y (.location _returnvalue))) (`KismetMathLibrary.MakeVector` (.x (.location _returnvalue_3)) (.y (.location _returnvalue_3))) _time 35.0)))
            (`self.K2_SetActorLocation` player (`KismetMathLibrary.MakeVector` _returnvalue_x _returnvalue_y (.z (.location _returnvalue))) false false)
            (`Controller.SetControlRotation` (`Pawn.GetController` player) (`KismetMathLibrary.RInterpTo_Constant` (.rotation _returnvalue) (.rotation _returnvalue_3) _time 35.0)))
          (:`Finished`
            (bind _asbp_first_person_character (cast `/Game/FirstPerson/Blueprints/BP_FirstPersonCharacter` player))
            (`/Game/FirstPerson/Blueprints/BP_FirstPersonCharacter.PushTreeDown` _asbp_first_person_character)
            (`KismetSystemLibrary.Delay` 1.55)
            (`FMODBlueprintStatics.PlayEventAtLocation` "/Game/FMOD/Events/OneShots/tree_falls.tree_falls" (`self.GetTransform`))
            (bind (_direction_2 _time_2) (`Timeline|Timeline` :!via `PlayFromStart`)
              (:`Update`
                (`SceneComponent.K2_SetRelativeRotation` (`self.TreeRootPoint`) (`KismetMathLibrary.RInterpTo_Constant` (`SceneComponent.RelativeRotation` (`self.TreeRootPoint`)) (struct :`Pitch` 90.0) _time_2 5.0) false false))
              (:`Finished`
                (set `self.TreeDown` true)
                (`GameplayStatics.PlayWorldCameraShake` "/Game/FirstPerson/Effects/CameraShake/BP_Tap_CamShake.BP_Tap_CamShake_C" _returnvalue_2 0.0 250.0)
                (`GameplayStatics.SpawnForceFeedbackAtLocation` "/Game/FirstPerson/Effects/HapticFeedback/FFE_Impact.FFE_Impact" _returnvalue_2 (struct) false 1.0 0.0 null)))))))))

(fn `UserConstructionScript`)