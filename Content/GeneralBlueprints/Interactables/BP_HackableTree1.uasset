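; Interactable tree that the player pushes over, usable only once.
; Interact runs a timeline that eases the player's horizontal position and view rotation toward the PlayerPosition0 marker.
; It then calls PushTreeDown on the first-person character and sets TreeDown after a short delay timed in code.
; Once TreeDown is set, Tick rotates TreeRootPoint at constant speed to the fallen angle.
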(event `self.ReceiveTick`
  (params (DeltaSeconds :type "Float (single-precision)"))
  (if (`self.TreeDown`)
    (`SceneComponent.K2_SetRelativeRotation` (`self.TreeRootPoint`) (`KismetMathLibrary.RInterpTo_Constant` (`SceneComponent.RelativeRotation` (`self.TreeRootPoint`)) (struct :`Pitch` 90.0) DeltaSeconds 90.0) false false)))

(event `InteractInterface.Interact`
  (params (player :type "HorrorTemplateCharacter Object Reference") (ElapsedSeconds :type "Float (single-precision)"))
  (bind _returnvalue (`self.GetTransform` player))
  (bind _returnvalue_2 (`SceneComponent.K2_GetComponentToWorld` (`self.PlayerPosition_0`)))
  (`/Engine/EditorBlueprintResources/StandardMacros.DoOnce` false
    (:`Completed`
      (if (not (`self.TreeDown`))
        (bind (_direction _time) (`Timeline|MovePLayer` :!via `PlayFromStart`)
          (:`Update`
            (bind (_returnvalue_x _returnvalue_y) (`KismetMathLibrary.BreakVector` (`KismetMathLibrary.VInterpTo_Constant` (`KismetMathLibrary.MakeVector` (.x (.location _returnvalue)) (.y (.location _returnvalue))) (`KismetMathLibrary.MakeVector` (.x (.location _returnvalue_2)) (.y (.location _returnvalue_2))) _time 35.0)))
            (`self.K2_SetActorLocation` player (`KismetMathLibrary.MakeVector` _returnvalue_x _returnvalue_y (.z (.location _returnvalue))) false false)
            (`Controller.SetControlRotation` (`Pawn.GetController` player) (`KismetMathLibrary.RInterpTo_Constant` (.rotation _returnvalue) (.rotation _returnvalue_2) _time 35.0)))
          (:`Finished`
            (bind _asbp_first_person_character (cast `/Game/FirstPerson/Blueprints/BP_FirstPersonCharacter` player))
            (`/Game/FirstPerson/Blueprints/BP_FirstPersonCharacter.PushTreeDown` _asbp_first_person_character)
            (`KismetSystemLibrary.Delay` 1.55)
            (set `self.TreeDown` true)))))))

(fn `UserConstructionScript`)