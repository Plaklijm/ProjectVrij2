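; BP_Core is an interactable core that stages an animated interaction with the first-person player.
; On Interact, it moves the player to the Loc component and turns their control rotation toward the Rot component.
; It then calls PlayCoreAnim on BP_FirstPersonCharacter and, through a DoOnce, plays the Core montage on its own skeletal mesh only the first time.
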(event `self.ReceiveBeginPlay`)

(event `InteractInterface.Interact`
  (params (player :type "HorrorTemplateCharacter Object Reference") (ElapsedSeconds :type "Float (single-precision)"))
  (`self.K2_SetActorLocation` player (`SceneComponent.K2_GetComponentLocation` (`self.Loc`)) false false)
  (`Controller.SetControlRotation` (`Pawn.GetController` player) (`KismetMathLibrary.FindLookAtRotation` (`self.K2_GetActorLocation` player) (`SceneComponent.K2_GetComponentLocation` (`self.Rot`))))
  (bind _asbp_first_person_character (cast `/Game/FirstPerson/Blueprints/BP_FirstPersonCharacter` player))
  (`/Game/FirstPerson/Blueprints/BP_FirstPersonCharacter.PlayCoreAnim` _asbp_first_person_character)
  (`/Engine/EditorBlueprintResources/StandardMacros.DoOnce` false
    (:`Completed`
      (`|PlayMontage` (`self.SkeletalMesh`) "/Game/Core.Core"))))

(fn `UserConstructionScript`)