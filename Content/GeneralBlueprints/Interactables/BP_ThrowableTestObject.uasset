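; BP_ThrowableTestObject is a test interactable that the first-person character picks up as a stone, then can throw or drop.
; Interact passes it to PickupStone, then destroys the actor.
; Throw detaches it and launches it once through a projectile component, while Drop detaches it and simulates physics for a short delay.
; Mesh hits emit a gameplay noise and switch on a point light, which throwing or finishing a drop switches off.
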(event `self.ReceiveBeginPlay`
  (`PrimitiveComponent.SetSimulatePhysics` (`self.Mesh`) false)
  (`ActorComponent.SetActive` (`self.PointLight`) false false))

(event `self.Mesh.OnComponentHit`
  (params (HitComponent :type "PrimitiveComponent Object Reference") (OtherActor :type "Actor Object Reference") (OtherComp :type "PrimitiveComponent Object Reference") (NormalImpulse :type "Vector Structure") (Hit :type "HitResult Structure (by ref)"))
  (`self.MakeNoise` 0.7 null (`self.K2_GetActorLocation`) 1000.0)
  (`ActorComponent.SetActive` (`self.PointLight`) true false))

(event `Throw`
  (params (Velocity :type "Vector Structure"))
  (bind _projectilecomponent (`self.ProjectileComponent`))
  (`/Engine/EditorBlueprintResources/StandardMacros.DoOnce` false
    (:`Completed`
      (set `MovementComponent.Velocity` Velocity _projectilecomponent)
      (`PrimitiveComponent.SetCollisionEnabled` (`self.Mesh`) "QueryAndPhysics")
      (`self.K2_DetachFromActor` "KeepWorld" "KeepWorld" "KeepWorld")
      (`ActorComponent.Activate` _projectilecomponent false)
      (`ActorComponent.SetActive` (`self.PointLight`) false false))))

(event `Drop`
  (`self.K2_DetachFromActor` "KeepWorld" "KeepWorld" "KeepWorld")
  (`PrimitiveComponent.SetCollisionEnabled` (`self.Mesh`) "QueryAndPhysics")
  (`PrimitiveComponent.SetSimulatePhysics` (`self.Mesh`) true)
  (`KismetSystemLibrary.Delay` 2.0)
  (`PrimitiveComponent.SetSimulatePhysics` (`self.Mesh`) false)
  (`ActorComponent.SetActive` (`self.PointLight`) false false))

(event `InteractInterface.Interact`
  (params (player :type "HorrorTemplateCharacter Object Reference") (ElapsedSeconds :type "Float (single-precision)"))
  (bind _asbp_first_person_character (cast `/Game/FirstPerson/Blueprints/BP_FirstPersonCharacter` player))
  (`/Game/FirstPerson/Blueprints/BP_FirstPersonCharacter.PickupStone` _asbp_first_person_character self)
  (`self.K2_DestroyActor`))

(fn `UserConstructionScript`)