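; BP_JuiceFlow is an animation notify state that turns juice flow on and off during a first-person character animation.
; On begin and end, it casts the mesh owner to BP_FirstPersonCharacter and calls StartFlow or StopFlow on that character's Tap.
; The flow lasts as long as the notify window, and nothing happens if the owner is another class.
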(fn `Received_NotifyBegin`
  (params (MeshComp :type "SkeletalMeshComponent Object Reference") (Animation :type "AnimSequenceBase Object Reference") (TotalDuration :type "Float (single-precision)") (EventReference :type "AnimNotifyEventReference Structure (by ref)"))
  (returns (ReturnValue :type Boolean))
  (bind _asbp_first_person_character (cast `/Game/FirstPerson/Blueprints/BP_FirstPersonCharacter` (`ActorComponent.GetOwner` MeshComp)))
  (`/Game/FirstPerson/Blueprints/BP_Tap.StartFlow` (`/Game/FirstPerson/Blueprints/BP_FirstPersonCharacter.Tap` _asbp_first_person_character))
  (return false))

(fn `Received_NotifyEnd`
  (params (MeshComp :type "SkeletalMeshComponent Object Reference") (Animation :type "AnimSequenceBase Object Reference") (EventReference :type "AnimNotifyEventReference Structure (by ref)"))
  (returns (ReturnValue :type Boolean))
  (bind _asbp_first_person_character (cast `/Game/FirstPerson/Blueprints/BP_FirstPersonCharacter` (`ActorComponent.GetOwner` MeshComp)))
  (`/Game/FirstPerson/Blueprints/BP_Tap.StopFlow` (`/Game/FirstPerson/Blueprints/BP_FirstPersonCharacter.Tap` _asbp_first_person_character))
  (return false))